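; BP_MyLobbyCharacter is a lobby character Blueprint that cycles through selectable character appearances.
; Its ChangeCharacter event advances CurrentCharacterIndex through the Characters array, wrapping to zero after the last entry, and assigns that entry as the SkeletalMesh component's asset.
; BeginPlay, overlap, Tick and the construction script are empty, so the mesh changes only when ChangeCharacter is called.
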(event Custom|Change%20Character
  (if (< (Variables|Default|GetcurrentCharacterIndex) (- (Utilities|Array|Length (Variables|Default|Getcharacters)) 1))
    (Math|Integer|IncrementInt (Variables|Default|GetcurrentCharacterIndex)
      (:%20%20
        _))
    (else
      (Variables|Default|SetcurrentCharacterIndex 0)))
  (Variables|/Script/Engine.SkeletalMeshComponent|SetSkeletalMeshAsset (Variables|Default|GetSkeletalMesh) (Utilities|Array|Get(acopy) (Variables|Default|Getcharacters) (Variables|Default|GetcurrentCharacterIndex))))

(event EventBeginPlay)

(event Collision|EventActorBeginOverlap
  (params (OtherActor :type Actor%20Object%20Reference)))

(event EventTick
  (params (DeltaSeconds :type Float%20%28single-precision%29)))

(fn ConstructionScript)