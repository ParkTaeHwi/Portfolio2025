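; BP_MyLobbyStage is a lobby stage actor that shows one skeletal mesh at a time from its Cubemesh array.
; BeginPlay takes the starting index from SetCubeIndex, which is defined outside this file, and applies that mesh.
; The StageChange event advances the index, wrapping to zero after the last entry, then swaps the mesh and calls LogCubeIndex.
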(event Custom|StageChange
  (if (< (Variables|Default|GetcurrentCubeIndex) (- (Utilities|Array|Length (Variables|Default|Getcubemesh)) 1))
    (Math|Integer|IncrementInt (Variables|Default|GetcurrentCubeIndex)
      (:%20%20
        _))
    (else
      (Variables|Default|SetcurrentCubeIndex 0)))
  (Variables|/Script/Engine.SkeletalMeshComponent|SetSkeletalMeshAsset (Variables|Default|GetSkeletalMesh) (Utilities|Array|Get(acopy) (Variables|Default|Getcubemesh) (Variables|Default|GetcurrentCubeIndex)))
  (Class|MyLobbyStage|LogCubeIndex))

(event Collision|EventActorBeginOverlap
  (params (OtherActor :type Actor%20Object%20Reference)))

(event EventTick
  (params (DeltaSeconds :type Float%20%28single-precision%29)))

(event EventBeginPlay
  (bind _returnvalue (Class|MyLobbyStage|SetCubeIndex))
  (Variables|Default|SetCurrentCubeIndex _returnvalue)
  (Variables|/Script/Engine.SkeletalMeshComponent|SetSkeletalMeshAsset (Variables|Default|GetSkeletalMesh) (Utilities|Array|Get(acopy) (Variables|Default|Getcubemesh) (Variables|Default|GetcurrentCubeIndex))))

(fn ConstructionScript)